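; BP_HouseActor is a house actor with a marker widget that shows how far away the player is when the house is the target.
; Every Tick sets the widget component's visibility from GetIsTarget.
; It also sends the truncated distance to player pawn 0, converted to meters with an "m" suffix, to the widget, even while the marker is hidden.
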(event `self.ReceiveTick`
  (params (DeltaSeconds :type "Float (single-precision)"))
  (`SceneComponent.SetVisibility` (`self.MarkerWidget`) (`self.GetIsTarget`) false)
  (message `/Game/BPI_Waypoint.SetDistanceText` (`WidgetComponent.GetUserWidgetObject` (`self.MarkerWidget`)) (`KismetTextLibrary.Conv_StringToText` (`KismetStringLibrary.Concat_StrStr` (`KismetStringLibrary.Conv_IntToString` (`KismetMathLibrary.FTrunc` (/ (`KismetMathLibrary.Vector_Distance` (`self.K2_GetActorLocation`) (`self.K2_GetActorLocation` (`GameplayStatics.GetPlayerPawn` 0))) 100.0))) "m"))))

(fn `UserConstructionScript`)